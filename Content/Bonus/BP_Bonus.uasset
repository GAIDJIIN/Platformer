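; BP_Bonus is a base pickup for the side-scroller that floats and spins until a character collects it.
; A timeline started at BeginPlay drives the Arrow component's relative height and yaw.
; When a SideScrollerCharacter overlaps the Bonus component, it calls TakeEffect, plays a sound and destroys itself.
; TakeEffect is empty here, leaving the actual effect undefined in this Blueprint.
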(event `self.ReceiveBeginPlay`
  (bind (_relativerotation_roll _relativerotation_pitch) (`KismetMathLibrary.BreakRotator` (`SceneComponent.RelativeRotation` (`self.Arrow`))))
  (bind (_direction _levitate _rotate) (`Timeline|TimelineLevitate`)
    (:`Update`
      (`SceneComponent.K2_SetRelativeTransform` (`self.Arrow`) (`KismetMathLibrary.MakeTransform` (`KismetMathLibrary.MakeVector` 0.0 0.0 _levitate) (`KismetMathLibrary.MakeRotator` _relativerotation_roll _relativerotation_pitch _rotate)) false false))))

(event `self.Bonus.OnComponentBeginOverlap`
  (params (OverlappedComponent :type "PrimitiveComponent Object Reference") (OtherActor :type "Actor Object Reference") (OtherComp :type "PrimitiveComponent Object Reference") (OtherBodyIndex :type Integer) (bFromSweep :type Boolean) (SweepResult :type "HitResult Structure (by ref)"))
  (bind _asside_scroller_character (cast `/Game/SideScrollerBP/Blueprints/SideScrollerCharacter` OtherActor))
  (`self.Take Effect` _asside_scroller_character)
  (`GameplayStatics.PlaySound2D` (`self.SoundBonus`) 1.0 1.0 0.0 null null)
  (`self.K2_DestroyActor`))

(event `Take Effect`
  (params (Character :type "/Game/SideScrollerBP/Blueprints/SideScrollerCharacter Object Reference")))

(fn `UserConstructionScript`)