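; BP_Trap is a pressure-triggered cone trap for the side-scroller character that damages and knocks the player upward.
; Overlapping the Box plays a button sound, waits an activation delay, then runs a timeline that animates the Trap's Z scale.
; Touching the Trap damages energy and points through the character's states component and launches it.
; Two boolean gates block retriggering and repeat hits, resetting when the timeline finishes.
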(event `self.Box.OnComponentBeginOverlap`
  (params (OverlappedComponent :type "PrimitiveComponent Object Reference") (OtherActor :type "Actor Object Reference") (OtherComp :type "PrimitiveComponent Object Reference") (OtherBodyIndex :type Integer) (bFromSweep :type Boolean) (SweepResult :type "HitResult Structure (by ref)"))
  (bind _trap (`self.Trap`))
  (bind (_relativescale3d_x _relativescale3d_y) (`KismetMathLibrary.BreakVector` (`SceneComponent.RelativeScale3D` _trap)))
  ;[1 1 1] TrapUp
  (cast `/Game/SideScrollerBP/Blueprints/SideScrollerCharacter` OtherActor)
  (if (`self.TrapChange`)
    (set `self.TrapChange` false)
    (`GameplayStatics.PlaySound2D` "/Game/Sounds/Step_on_Button.Step_on_Button" 1.0 1.0 0.0 null null)
    (`KismetSystemLibrary.Delay` (`self.TimeActivationTrap`))
    (`GameplayStatics.PlaySoundAtLocation` "/Game/Sounds/Trap.Trap" (`self.K2_GetActorLocation`) (struct) 1.0 1.0 0.0 null null null)
    (bind (_direction _trap_2) (`Timeline|TimeForTrap` :!via `PlayFromStart`)
      (:`Update`
        (`SceneComponent.SetRelativeScale3D` _trap (`KismetMathLibrary.MakeVector` _relativescale3d_x _relativescale3d_y _trap_2)))
      (:`Finished`
        (set `self.TrapChange` true)
        (set `self.TrapDamage` true)))))

(event `self.Trap.OnComponentBeginOverlap`
  (params (OverlappedComponent :type "PrimitiveComponent Object Reference") (OtherActor :type "Actor Object Reference") (OtherComp :type "PrimitiveComponent Object Reference") (OtherBodyIndex :type Integer) (bFromSweep :type Boolean) (SweepResult :type "HitResult Structure (by ref)"))
  ;[1 1 1] TrapDamage
  (bind _asside_scroller_character (cast `/Game/SideScrollerBP/Blueprints/SideScrollerCharacter` OtherActor))
  (if (`self.TrapDamage`)
    (set `self.TrapDamage` false)
    (`GameplayStatics.PlaySound2D` "/Game/Sounds/Damage.Damage" 1.0 1.0 0.0 null null)
    (`/Game/SideScrollerBP/Blueprints/BPС_States.Damage` (`/Game/SideScrollerBP/Blueprints/SideScrollerCharacter.BPС_States` _asside_scroller_character) 10 100)
    (`Character.LaunchCharacter` _asside_scroller_character (0.0 0.0 400.0) false false)))

(fn `UserConstructionScript`)