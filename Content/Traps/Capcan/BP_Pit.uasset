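; Trap Blueprint for the side-scroller character that springs after a delay and can act as a pit.
; Box overlap plays a button sound, waits TimeActivation, then runs the Capcan timeline to pitch Arrow, hiding Floor and its collision when IsPit is set.
; Leaving starts a looping timer, cleared on re-entry, that counts up to TimeActivation, then restores the floor and reverses Capcan.
; DoorOpen blocks retriggering until the reverse finishes.
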(event `self.Box.OnComponentBeginOverlap`
  (params (OverlappedComponent :type "PrimitiveComponent Object Reference") (OtherActor :type "Actor Object Reference") (OtherComp :type "PrimitiveComponent Object Reference") (OtherBodyIndex :type Integer) (bFromSweep :type Boolean) (SweepResult :type "HitResult Structure (by ref)"))
  ;[1 1 1] PitLogic
  (cast `/Game/SideScrollerBP/Blueprints/SideScrollerCharacter` OtherActor)
  (`KismetSystemLibrary.K2_ClearAndInvalidateTimerHandle` (`self.TimerHandle`))
  (set `self.Time` 0.0)
  (if (`self.DoorOpen`)
    (set `self.DoorOpen` false)
    (`GameplayStatics.PlaySound2D` "/Game/Sounds/Step_on_Button.Step_on_Button" 1.0 1.0 0.0 null null)
    (`KismetSystemLibrary.Delay` (`self.TimeActivation`))
    (`GameplayStatics.PlaySoundAtLocation` null (`self.K2_GetActorLocation`) (struct) 1.0 1.0 0.0 null null null)
    (`self.HideFloor` (`self.IsPit?`))
    (bind (_direction _trap) (`Timeline|Capcan` :!via `PlayFromStart` :!label _label)
      (:`Update`
        (`SceneComponent.K2_SetRelativeRotation` (`self.Arrow`) (`KismetMathLibrary.MakeRotator` 0.0 _trap) false false))
      (:`Finished`
        (switch `ETimelineDirection` _direction
          (:`Backward`
            (set `self.DoorOpen` true)))))))

(event `self.Box.OnComponentEndOverlap`
  (params (OverlappedComponent :type "PrimitiveComponent Object Reference") (OtherActor :type "Actor Object Reference") (OtherComp :type "PrimitiveComponent Object Reference") (OtherBodyIndex :type Integer))
  ;[1 1 1] PitLogic
  (bind _returnvalue (`KismetSystemLibrary.K2_SetTimerDelegate` (delegate `Timer`) 0.75 true))
  (set `self.TimerHandle` _returnvalue))

(event `Timer`
  ;[1 1 1] PitLogic
  (if (>= (`self.Time`) (`self.TimeActivation`))
    (`KismetSystemLibrary.K2_ClearAndInvalidateTimerHandle` (`self.TimerHandle`))
    (`self.ShowFloor` (`self.IsPit?`))
    (goto _label :!via `Reverse`)
    (else
      (set `self.Time` (+ (`self.Time`) 0.5)))))

(fn `HideFloor`
  (params (`IsPit?` :type Boolean))
  (bind _floor (`self.Floor`))
  (if `IsPit?`
    (`SceneComponent.SetVisibility` _floor false false)
    (`PrimitiveComponent.SetCollisionEnabled` _floor "NoCollision")))

(fn `ShowFloor`
  (params (`IsPit?` :type Boolean))
  (bind _floor (`self.Floor`))
  (if `IsPit?`
    (`SceneComponent.SetVisibility` _floor true false)
    (`PrimitiveComponent.SetCollisionEnabled` _floor "QueryAndPhysics")))

(fn `UserConstructionScript`)