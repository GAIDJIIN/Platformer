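; BP_Capcan is a side-scroller trap that repeatedly hurts the player character standing in its TrapDamage volume.
; On overlap by a SideScrollerCharacter it plays a sound, applies energy damage and point loss through the character's BPСStates component, and launches it upward.
; A looping half-second timer repeats that hit until any overlap with the volume ends, which clears the timer.
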(event `self.TrapDamage.OnComponentBeginOverlap`
  (params (OverlappedComponent :type "PrimitiveComponent Object Reference") (OtherActor :type "Actor Object Reference") (OtherComp :type "PrimitiveComponent Object Reference") (OtherBodyIndex :type Integer) (bFromSweep :type Boolean) (SweepResult :type "HitResult Structure (by ref)"))
  ;[1 1 1] Capcan
  (bind _asside_scroller_character (cast `/Game/SideScrollerBP/Blueprints/SideScrollerCharacter` OtherActor))
  (`GameplayStatics.PlaySound2D` "/Game/Sounds/Damage.Damage" 1.0 1.0 0.0 null null)
  (`/Game/SideScrollerBP/Blueprints/BPС_States.Damage` (`/Game/SideScrollerBP/Blueprints/SideScrollerCharacter.BPС_States` _asside_scroller_character) 5 50)
  (`Character.LaunchCharacter` _asside_scroller_character (0.0 0.0 400.0) false false)
  (bind _returnvalue (`KismetSystemLibrary.K2_SetTimerDelegate` (delegate `Damage`) 0.5 true))
  (set `self.DamageTimer` _returnvalue))

(event `Damage`
  ;[1 1 1] Capcan
  (`GameplayStatics.PlaySound2D` "/Game/Sounds/Damage.Damage" 1.0 1.0 0.0 null null)
  (`/Game/SideScrollerBP/Blueprints/BPС_States.Damage` (`/Game/SideScrollerBP/Blueprints/SideScrollerCharacter.BPС_States` (stale `self.TrapDamage.OnComponentBeginOverlap` _asside_scroller_character)) 5 50)
  (`Character.LaunchCharacter` (stale `self.TrapDamage.OnComponentBeginOverlap` _asside_scroller_character) (0.0 0.0 400.0) false false))

(event `self.TrapDamage.OnComponentEndOverlap`
  (params (OverlappedComponent :type "PrimitiveComponent Object Reference") (OtherActor :type "Actor Object Reference") (OtherComp :type "PrimitiveComponent Object Reference") (OtherBodyIndex :type Integer))
  ;[1 1 1] Capcan
  (`KismetSystemLibrary.K2_ClearAndInvalidateTimerHandle` (`self.DamageTimer`)))

(fn `UserConstructionScript`
  (`parent.UserConstructionScript`))