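; BP_Launcher is a trap that fires a rocket when the SideScrollerCharacter crosses its laser trigger.
; The overlap plays a sound, hides the laser and disables the box collision, then a timer spawns BP_Rocket with the configured speed.
; The laser and collision return after the spawn time plus the activation time.
; The construction script sizes the beam and trigger from HeightLaser.
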(event `self.Box.OnComponentBeginOverlap`
  (params (OverlappedComponent :type "PrimitiveComponent Object Reference") (OtherActor :type "Actor Object Reference") (OtherComp :type "PrimitiveComponent Object Reference") (OtherBodyIndex :type Integer) (bFromSweep :type Boolean) (SweepResult :type "HitResult Structure (by ref)"))
  ;[1 1 1] LaucnhSpear
  (cast `/Game/SideScrollerBP/Blueprints/SideScrollerCharacter` OtherActor)
  (`GameplayStatics.PlaySoundAtLocation` "/Game/Sounds/Lazer.Lazer" (`self.K2_GetActorLocation`) (struct) 1.0 1.0 0.0 null null null)
  (`KismetSystemLibrary.K2_SetTimerDelegate` (delegate `LaunсhRocket`) (`self.Time Spawning`))
  (`self.VisibleLaser`))

(event `LaunсhRocket`
  ;[1 1 1] LaucnhSpear
  (bind _returnvalue (`|SpawnActorFromClass` "/Game/Traps/RocketLauncher/BP_Rocket.BP_Rocket_C" (`KismetMathLibrary.MakeTransform` (`self.K2_GetActorLocation`) (`self.K2_GetActorRotation`)) "Undefined" "OverrideRootScale" null null))
  (set `/Game/Traps/RocketLauncher/BP_Rocket.RocketSpeed` (`self.Rocket Speed`) _returnvalue))

(event `VisibleLaser`
  ;[1 1 1] VisibleLaser
  (`SceneComponent.SetVisibility` (`self.ParticleSystem`) false false)
  (`PrimitiveComponent.SetCollisionEnabled` (`self.Box`) "NoCollision")
  (`KismetSystemLibrary.Delay` (+ (`self.Time Spawning`) (`self.TimeActivationLauncher`)))
  (`SceneComponent.SetVisibility` (`self.ParticleSystem`) true false)
  (`PrimitiveComponent.SetCollisionEnabled` (`self.Box`) "QueryOnly"))

(fn `HideLazer`
  (`SceneComponent.SetVisibility` (`self.ParticleSystem`) false false)
  (`PrimitiveComponent.SetCollisionEnabled` (`self.Box`) "NoCollision"))

(fn `ShowLazer`)

(fn `UserConstructionScript`
  (bind _height_laser (`self.Height Laser`))
  (bind (_relativelocation_x _relativelocation_y _relativelocation_z) (`KismetMathLibrary.BreakVector` (`SceneComponent.RelativeLocation` (`self.Box`))))
  (bind (_relativescale3d_x _relativescale3d_y _relativescale3d_z) (`KismetMathLibrary.BreakVector` (`SceneComponent.RelativeScale3D` (`self.Box`))))
  (`SceneComponent.SetRelativeScale3D` (`self.ParticleSystem`) (`KismetMathLibrary.MakeVector` _height_laser 0.65 0.65))
  (`SceneComponent.SetRelativeScale3D` (`self.Box`) (`KismetMathLibrary.MakeVector` 0.125 0.125 (* _height_laser _relativescale3d_z)))
  (`SceneComponent.K2_SetRelativeLocation` (`self.Box`) (`KismetMathLibrary.MakeVector` 0.0 0.0 (* _height_laser _relativelocation_z)) false false))