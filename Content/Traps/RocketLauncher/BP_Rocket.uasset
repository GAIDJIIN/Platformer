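; Rocket projectile for the rocket launcher trap that explodes on impact and damages the side-scroller character.
; A fast looping timer, started on BeginPlay with a launch sound, moves the Box along its local Z with sweep.
; A Box hit stops the timer, plays explosion effects and destroys the rocket.
; Character hits also apply damage through BPСStates and launch the player upward and along the sweep's Y direction.
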(event `self.ReceiveBeginPlay`
  ;[1 1 1] MoveSpear
  (`GameplayStatics.PlaySoundAtLocation` "/Game/Sounds/New_Launch_Rocket.New_Launch_Rocket" (`self.K2_GetActorLocation`) (struct) 1.0 1.0 0.0 null null null)
  (bind _returnvalue (`KismetSystemLibrary.K2_SetTimerDelegate` (delegate `MoveSpear`) 0.001 true))
  (set `self.Time` _returnvalue))

(event `MoveSpear`
  ;[1 1 1] MoveSpear
  (`SceneComponent.K2_AddLocalOffset` (`self.Box`) (`KismetMathLibrary.MakeVector` 0.0 0.0 (`self.RocketSpeed`)) true false))

(event `self.Box.OnComponentHit`
  (params (HitComponent :type "PrimitiveComponent Object Reference") (OtherActor :type "Actor Object Reference") (OtherComp :type "PrimitiveComponent Object Reference") (NormalImpulse :type "Vector Structure") (Hit :type "HitResult Structure (by ref)"))
  (bind (_returnvalue_x _returnvalue_y) (`KismetMathLibrary.BreakVector` (- Hit_TraceStart Hit_TraceEnd)))
  (bind _hit_location (`self.Hit Location`))
  ;[1 1 1] HitSpear
  (set `self.Hit Location` Hit_Location)
  (set `self.LaunchVector` (* -300 (/ _returnvalue_y (`KismetMathLibrary.Abs` _returnvalue_y))))
  (`KismetSystemLibrary.K2_ClearAndInvalidateTimerHandle` (`self.Time`))
  (bind _asside_scroller_character (cast `/Game/SideScrollerBP/Blueprints/SideScrollerCharacter` OtherActor)
    (:`then`
      (`GameplayStatics.PlaySound2D` "/Game/Sounds/Damage_SC.Damage_SC" 1.0 1.0 0.0 null null)
      (`GameplayStatics.SpawnEmitterAtLocation` "/Game/StarterContent/Particles/P_Explosion.P_Explosion" (+ (`self.K2_GetActorLocation` _asside_scroller_character) (0.0 0.0 30.0)) (struct) (0.75 0.75 0.75))
      (`self.K2_DestroyActor`)
      (`/Game/SideScrollerBP/Blueprints/BPС_States.Damage` (`/Game/SideScrollerBP/Blueprints/SideScrollerCharacter.BPС_States` _asside_scroller_character) 10 100)
      (`Character.LaunchCharacter` _asside_scroller_character (`KismetMathLibrary.MakeVector` 0.0 (`self.LaunchVector`) 400.0) false false))
    (:`CastFailed`
      (`GameplayStatics.PlaySoundAtLocation` "/Game/Sounds/Rocket_Boom.Rocket_Boom" _hit_location (struct) 1.0 1.0 0.0 null null null)
      (`GameplayStatics.SpawnEmitterAtLocation` "/Game/StarterContent/Particles/P_Explosion.P_Explosion" _hit_location)
      (`self.K2_DestroyActor`))))

(fn `UserConstructionScript`)